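; BP_HoverComponent is a hover suspension point for a BP_VehicleBase owner, pushing the vehicle away from surfaces beneath it.
; Each tick it line-traces along its local down vector up to HoverDistance, with debug drawing on.
; On a hit it applies a spring-damper force at its location on the vehicle's root primitive, deriving damping from the change in hover delta.
; It also stores normalized Compression, zeroed on a miss.
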(event EventBeginPlay
  (bind _asbp_vehicle_base (Utilities|Casting|CastToBP_VehicleBase (Components|GetOwner)))
  (Variables|Default|SetParentVehicle _asbp_vehicle_base))

(event EventTick
  (params (DeltaSeconds :type Float%20%28single-precision%29))
  (bind _returnvalue (Transformation|GetWorldLocation))
  (bind _hoverdistance (Variables|Default|GetHoverDistance))
  (Utilities|IsValid (Variables|Default|GetParentVehicle)
    (:Is%20Valid
      (bind (_outhit _returnvalue_2) (Collision|LineTraceByChannel _returnvalue (- _returnvalue (* (Math|Vector|GetUpVector) (Variables|Default|GetHoverDistance))) "TraceTypeQuery1" false 0 "ForOneFrame" true "(R=0.000000,G=0.094607,B=1.000000,A=1.000000)"))
      (if _returnvalue_2
        (Variables|Default|SetCompression (/ (- _hoverdistance (.Distance (Collision|BreakHitResult _outhit))) _hoverdistance))
        (bind _output_get (Variables|Default|SetHoverDelta (- _hoverdistance (.Distance (Collision|BreakHitResult _outhit)))))
        (Class|PrimitiveComponent|AddForceatLocation (.AsPrimitive%20Component (Utilities|Casting|CastToPrimitiveComponent (Variables|/Script/Engine.Actor|GetRootComponent (Variables|Default|GetParentVehicle)))) (* (+ (* (/ (- _output_get (Variables|Default|GetPrevHoverDelta)) (Utilities|Time|GetWorldDeltaSeconds)) (Variables|Default|GetDampingCoefficient)) (* _output_get (Variables|Default|GetSpringCoefficient))) (Math|Vector|GetUpVector)) (Transformation|GetWorldLocation) "None")
        (Variables|Default|SetPrevHoverDelta (Variables|Default|GetHoverDelta))
        (else
          (Variables|Default|SetCompression 0.0))))))